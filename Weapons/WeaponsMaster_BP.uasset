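; WeaponsMaster_BP is a weapon base for a third-person shooter that handles firing, aiming and attachment to its owning pawn.
; Start and stop fire route clients through server calls, with authority toggling WantsToFire.
; On fire start, CameraAim traces from the muzzle toward the controller's camera aim point, and an explosion emitter spawns at AimVector.
; The weapon snaps to the pawn's hand socket, deferring until OwningPawn replicates if needed.
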(event `Server_Startfire`
  (`self.StartFire`))

(event `Server_StopFire`
  (`self.StopFire`))

(fn `AttachToOwnerHolster`
  (bind _owning_pawn (`self.Owning Pawn`))
  (`/Engine/EditorBlueprintResources/StandardMacros.IsValid` _owning_pawn
    (:`Is Valid`
      (`SceneComponent.K2_AttachToComponent` (`self.WeaponMesh`) (`Character.Mesh` _owning_pawn) (`/Game/ThirdPersonBP/Blueprints/ThirdPersonCharacter.RHandWeaponSocket` _owning_pawn) "SnapToTarget" "SnapToTarget" "KeepRelative" true)
      (set `/Game/ThirdPersonBP/Blueprints/ThirdPersonCharacter.EquippedWeapon` self _owning_pawn))
    (:`Is Not Valid`
      (set `self.NeedsAttachedUpdateOnOwnerRep` true))))

(fn `CameraAim`
  (returns (NewParam :type Boolean))
  (bind _owning_pawn (`self.Owning Pawn`))
  (bind _astpsplayer_controller (`/Game/ThirdPersonBP/Blueprints/ThirdPersonCharacter.GetCastedOwner` _owning_pawn))
  (bind _returnvalue (+ (* (`/Game/Blueprints/TPSPlayerController.AimVector` _astpsplayer_controller) 100000.0) (`/Game/Blueprints/TPSPlayerController.ViewPoint` _astpsplayer_controller)))
  (set `self.AimVector` (`KismetMathLibrary.GetForwardVector` (`Pawn.GetBaseAimRotation` _owning_pawn)))
  (bind _outhit (`KismetSystemLibrary.LineTraceSingle` (`self.GetMuzzleLocation`) _returnvalue "TraceTypeQuery1"))
  (bind (_bblockinghit _binitialoverlap _time _distance _location) (`GameplayStatics.BreakHitResult` _outhit))
  (set `self.AimVector` (`KismetMathLibrary.SelectVector` _location (- _returnvalue (`self.GetMuzzleLocation`)) _bblockinghit))
  (return false))

(fn `GetMuzzleLocation`
  (returns (MuzzleLocation :type "Vector Structure"))
  (return (`SceneComponent.GetSocketLocation` (`self.WeaponMesh`) (`self.MuzzleSocket`))))

(fn `OnRep_Owning Pawn`
  (bind _owning_pawn (`self.Owning Pawn`))
  (if (and (`self.NeedsAttachedUpdateOnOwnerRep`) (`KismetSystemLibrary.IsValid` (`self.Owning Pawn`)))
    (set `self.NeedsAttachedUpdateOnOwnerRep` false)
    (`/Engine/EditorBlueprintResources/ActorMacros.Switch Has Authority`
      (:`Remote`
        (if (== (`/Game/ThirdPersonBP/Blueprints/ThirdPersonCharacter.EquippedWeapon` _owning_pawn) self)
          _
          (elif (== self (`/Game/ThirdPersonBP/Blueprints/ThirdPersonCharacter.GetHolstedWeapons` _owning_pawn (`self.SlotType`)))
            (`self.AttachToOwnerHolster`)))))))

(fn `SetOwningPawn`
  (params (`Owning Pawn` :type "/Game/ThirdPersonBP/Blueprints/ThirdPersonCharacter Object Reference"))
  (if (!= `Owning Pawn` (`self.Owning Pawn`))
    (bind _output_get (set `self.Owning Pawn` `Owning Pawn`))
    (`self.SetOwner` _output_get)))

(fn `StartFire`
  (`/Engine/EditorBlueprintResources/ActorMacros.Switch Has Authority`
    (:`Authority`
      (if (not (`self.WantsToFire`))
        (set `self.WantsToFire` true)
        (`self.CameraAim`)
        (`GameplayStatics.SpawnEmitterAtLocation` "/Game/StarterContent/Particles/P_Explosion.P_Explosion" (`self.AimVector`))))
    (:`Remote`
      (`self.Server_Startfire`))))

(fn `StopFire`
  (`/Engine/EditorBlueprintResources/ActorMacros.Switch Has Authority`
    (:`Authority`
      (if (`self.WantsToFire`)
        (set `self.WantsToFire` false)))
    (:`Remote`
      (`self.Server_StopFire`))))

(fn `UserConstructionScript`)